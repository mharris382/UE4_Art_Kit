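; BP_Skybox is a sky actor that displays a configurable cubemap on its sky static mesh.
; The construction script creates a dynamic instance of M_CustomSkybox and feeds it the Cubemap and Intensity Multiplier variables.
; It then assigns the same cubemap to the referenced Skylight, if valid, keeping visible sky and skylight source matched.
; The event graph holds only unused stubs, with no runtime logic.
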(event EventBeginPlay)

(event Collision|EventActorBeginOverlap
  (params (OtherActor :type Actor%20Object%20Reference)))

(event EventTick
  (params (DeltaSeconds :type Float%20%28single-precision%29)))

(fn ConstructionScript
  (bind _returnvalue (Rendering|Material|CreateDynamicMaterialInstance (Variables|Default|GetSkyStaticMesh) 0 "/Game/Sky/M_CustomSkybox.M_CustomSkybox" "None" :!class /Script/Engine.PrimitiveComponent))
  (bind _output_get (Variables|Default|Setskybox%20material _returnvalue))
  (Rendering|Material|SetTextureParameterValue _output_get "Cubemap" (Variables|Default|GetCubemap))
  (Rendering|Material|SetScalarParameterValue (Variables|Default|Getskybox%20material) "Intensity Multiplier" (Variables|Default|Getintensity%20multiplier) :!class /Script/Engine.MaterialInstanceDynamic)
  (Utilities|AssignCubemaptoSkylight))